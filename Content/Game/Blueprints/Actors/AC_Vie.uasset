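; Health component (AC_Vie) that tracks current life and a death flag for the actor that owns it.
; Damage and heal events adjust life only while not dead, and a reset event clears the flag and restores maximum life.
; All three route through UpdateVieEtNotif, which clamps the value, broadcasts QandVieChange, then sets the death flag and broadcasts QuandMort when life reaches zero.
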(event `/Game/Game/Blueprints/BPI_PrendDomage.PrendDomage`
  (params (PrendDomage :type "Float (double-precision)"))
  (if (not (`self.MortT/F`))
    (`self.UpdateVieEtNotif` (- (`self.VieActuel`) PrendDomage))))

(event `/Game/Game/Blueprints/BPI_PrendDomage.GagneVie`
  (params (Gagne :type "Float (double-precision)"))
  (if (not (`self.MortT/F`))
    (`self.UpdateVieEtNotif` (+ (`self.VieActuel`) Gagne))))

(event `/Game/Game/Blueprints/BPI_PrendDomage.ResetVie`
  (set `self.MortT/F` false)
  (`self.UpdateVieEtNotif` (`self.MaxVie`)))

(fn `UpdateVieEtNotif`
  (params (NouvelVie :type "Float (double-precision)"))
  (bind _output_get (set `self.VieActuel` (`KismetMathLibrary.FClamp` NouvelVie 0.0 (`self.MaxVie`))))
  (`self.QandVieChange` _output_get (`self.MaxVie`))
  (if (<= (`self.VieActuel`) 0.0)
    (bind _output_get_2 (set `self.MortT/F` true))
    (`self.QuandMort` _output_get_2)
    (else
      (set `self.MortT/F` false))))