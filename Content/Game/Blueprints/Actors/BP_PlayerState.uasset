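; Player state Blueprint that keeps the player's health persistent through the game instance and triggers respawn on death.
; On BeginPlay it either restores current and max health from BP_GameInstance or, on first initialization, resets the AC_Vie component and sets the DebutVieGI flag.
; Health change events write both values back to the game instance, while the death event asks BP_ThirdPersonGameMode to respawn player controller 0.
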(event `self.ReceiveBeginPlay`
  (bind _asbp_game_instance (cast `/Game/Game/Blueprints/BP_GameInstance` (`GameplayStatics.GetGameInstance`)))
  (bind _output_get (set `self.RefGameInstance` _asbp_game_instance))
  (if (`/Game/Game/Blueprints/BP_GameInstance.DebutVie_GI` _output_get)
    (`self.LoadVieFromGameInstance`)
    (else
      (`/Game/Game/Blueprints/Actors/AC_Vie.ResetVie` (`self.AC_Vie`))
      (set `/Game/Game/Blueprints/BP_GameInstance.DebutVie_GI` true _output_get))))

(event `self.AC_Vie.QandVieChange`
  (params (VieActuel :type "Float (double-precision)") (MaxVIe :type "Float (double-precision)"))
  (`self.SaveVieActuel` VieActuel)
  (`self.SaveMaxVie` MaxVIe))

(event `self.AC_Vie.QuandMort`
  (params (`MortT/F` :type Boolean))
  (bind _asbp_third_person_game_mode (cast `/Game/Game/Blueprints/GameModes/BP_ThirdPersonGameMode` (`GameplayStatics.GetGameMode`)))
  (`/Game/Game/Blueprints/GameModes/BP_ThirdPersonGameMode.StartRespawn` _asbp_third_person_game_mode (`GameplayStatics.GetPlayerController` 0)))

(fn `LoadVieFromGameInstance`
  (bind _output_get (set `/Game/Game/Blueprints/Actors/AC_Vie.MaxVie` (`/Game/Game/Blueprints/BP_GameInstance.MaxVie_GI` (`self.RefGameInstance`)) (`self.AC_Vie`)))
  (bind _output_get_2 (set `/Game/Game/Blueprints/Actors/AC_Vie.VieActuel` (`/Game/Game/Blueprints/BP_GameInstance.VieAcutel_GI` (`self.RefGameInstance`)) (`self.AC_Vie`)))
  (`/Game/Game/Blueprints/Actors/AC_Vie.QandVieChange` (`self.AC_Vie`) _output_get_2 _output_get))

(fn `SaveMaxVie`
  (params (NewMaxVie :type "Float (double-precision)"))
  (set `/Game/Game/Blueprints/BP_GameInstance.MaxVie_GI` NewMaxVie (`self.RefGameInstance`)))

(fn `SaveVieActuel`
  (params (NewVie :type "Float (double-precision)"))
  (set `/Game/Game/Blueprints/BP_GameInstance.VieAcutel_GI` NewVie (`self.RefGameInstance`)))

(fn `UserConstructionScript`)