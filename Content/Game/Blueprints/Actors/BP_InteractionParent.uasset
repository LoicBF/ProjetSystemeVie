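; BP_InteractionParent is a base actor for interactable objects, combining a mesh, a sphere trigger and a UI component.
; The construction script applies exposed mesh, transform, trigger radius and location, and UI position settings to those components.
; Trigger overlaps register or unregister the actor with BP_ThirdPersonCharacter.
; ToggleUI sets the prompt's visibility, and Interact stores the interacting character and prints a placeholder message.
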(event `self.InteractTrigger.OnComponentBeginOverlap`
  (params (OverlappedComponent :type "PrimitiveComponent Object Reference") (OtherActor :type "Actor Object Reference") (OtherComp :type "PrimitiveComponent Object Reference") (OtherBodyIndex :type Integer) (bFromSweep :type Boolean) (SweepResult :type "HitResult Structure (by ref)"))
  ; Trigger Overlap
  (bind _asbp_third_person_character (cast `/Game/Game/Blueprints/Pawns_Characters/Player/BP_ThirdPersonCharacter` OtherActor))
  (`/Game/Game/Blueprints/Pawns_Characters/Player/BP_ThirdPersonCharacter.AddInteraction` _asbp_third_person_character self))

(event `self.InteractTrigger.OnComponentEndOverlap`
  (params (OverlappedComponent :type "PrimitiveComponent Object Reference") (OtherActor :type "Actor Object Reference") (OtherComp :type "PrimitiveComponent Object Reference") (OtherBodyIndex :type Integer))
  ; Trigger Overlap
  (bind _asbp_third_person_character (cast `/Game/Game/Blueprints/Pawns_Characters/Player/BP_ThirdPersonCharacter` OtherActor))
  (`/Game/Game/Blueprints/Pawns_Characters/Player/BP_ThirdPersonCharacter.RemouveInteration` _asbp_third_person_character self))

(fn `Interact`
  (params (Character :type "/Game/Game/Blueprints/Pawns_Characters/Player/BP_ThirdPersonCharacter Object Reference"))
  (set `self.Character` Character)
  (`KismetSystemLibrary.PrintString` "Interaction"))

(fn `SetupMesh`
  ; SetupMesh - Transforme
  (`StaticMeshComponent.SetStaticMesh` (`self.InteractMesh`) (`self.InteractionMesh`))
  (`SceneComponent.K2_SetRelativeTransform` (`self.InteractMesh`) (`self.MeshTransform`) false false))

(fn `SetupTrigger`
  ; SetupTrigger - Location
  (`SphereComponent.SetSphereRadius` (`self.InteractTrigger`) (`self.TriggerZone`) true)
  (`SceneComponent.K2_SetRelativeLocation` (`self.InteractTrigger`) (`self.TriggerLacation`) false false))

(fn `SetupUI`
  ; SetupUI - Location
  (`SceneComponent.K2_SetRelativeLocation` (`self.InteractUI`) (`self.UILocation`) false false))

(fn `ToggleUI`
  (params (`UIT/F` :type Boolean))
  ; set visible
  (`SceneComponent.SetVisibility` (`self.InteractUI`) `UIT/F` false))

(fn `UserConstructionScript`
  ; Setup Tout le systeme
  (`self.SetupMesh`)
  (`self.SetupTrigger`)
  (`self.SetupUI`))